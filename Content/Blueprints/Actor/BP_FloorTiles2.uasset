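; Runner floor tile, apparently a child of a parent tile class, that places launch pads and recycles itself as the player passes.
; BeginPlay spawns a BP_LaunchPad at each of three jump points, as the random roll is fixed to zero.
; EndTrigger asks RunnerGM for a new tile and, if the character lives, destroys this tile and its tracked pickups, blockers and launchers.
; Tick derives the Jump flag from IntResult.
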(event `self.ReceiveTick`
  (params (DeltaSeconds :type "Float (single-precision)"))
  (`parent.ReceiveTick` DeltaSeconds)
  (if (>= (`self.IntResult`) 1)
    (set `self.Jump?` false)
    (else
      (set `self.Jump?` true))))

(event `self.ReceiveBeginPlay`
  (`parent.ReceiveBeginPlay`)
  (for _array_element (`|MakeArray` (`self.JumpL`) (`self.JumpM`) (`self.JumpR`))
    (switch `int` (`KismetMathLibrary.RandomIntegerInRange` 0)
      (:`0`
        (`/Engine/EditorBlueprintResources/StandardMacros.Do N` 3
          (:`Exit`
            (`self.Spawn Launcher` (`SceneComponent.K2_GetComponentToWorld` _array_element))))))))

(event `Spawn Launcher`
  (params (SpawnTransform :type "Transform Structure"))
  (bind _returnvalue (`|SpawnActorFromClass` "/Game/Blueprints/Actor/BP_LaunchPad.BP_LaunchPad_C" SpawnTransform "Undefined" "OverrideRootScale" null null))
  (`KismetArrayLibrary.Array_Add` (`self.Launcher`) _returnvalue))

(event `self.EndTrigger.OnComponentBeginOverlap`
  (params (OverlappedComponent :type "PrimitiveComponent Object Reference") (OtherActor :type "Actor Object Reference") (OtherComp :type "PrimitiveComponent Object Reference") (OtherBodyIndex :type Integer) (bFromSweep :type Boolean) (SweepResult :type "HitResult Structure (by ref)"))
  (bind _asmy_char (cast `/Game/Blueprints/MyChar` OtherActor))
  (bind _output_get (set `self.MyCharRef` _asmy_char))
  (bind _asrunner_gm (cast `/Game/Blueprints/GameMode/RunnerGM` (`GameplayStatics.GetGameMode`)))
  (`/Game/Blueprints/GameMode/RunnerGM.AddFloorTile` _asrunner_gm)
  (if (not (`/Game/Blueprints/MyChar.IsDead` _output_get))
    (`|ExecutionSequence`
      (:`then_0`
        (`self.K2_DestroyActor`))
      (:`then_1`
        (for _array_element (`self.Pickups`)
          (`/Engine/EditorBlueprintResources/StandardMacros.IsValid` _array_element
            (:`Is Valid`
              (`self.K2_DestroyActor` _array_element))))
        (for _array_element_2 (`self.Blocker1`)
          (`/Engine/EditorBlueprintResources/StandardMacros.IsValid` _array_element_2
            (:`Is Valid`
              (`self.K2_DestroyActor` _array_element_2))))
        (for _array_element_3 (`self.Blocker2`)
          (`/Engine/EditorBlueprintResources/StandardMacros.IsValid` _array_element_3
            (:`Is Valid`
              (`self.K2_DestroyActor` _array_element_3))))
        (for _array_element_4 (`self.Launcher`)
          (`/Engine/EditorBlueprintResources/StandardMacros.IsValid` _array_element_4
            (:`Is Valid`
              (`self.K2_DestroyActor` _array_element_4))))))))

(fn `UserConstructionScript`
  (`parent.UserConstructionScript`))