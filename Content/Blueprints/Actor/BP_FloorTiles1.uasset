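; A floor tile for an endless runner that fills its three lanes and recycles itself as the player advances.
; On BeginPlay each lane randomly gets a pickup or one of two blocker types, with DoN capping each blocker type.
; EndTrigger asks RunnerGM for another tile, then destroys this tile and its spawned actors if MyChar is alive.
; DeadTrigger kills MyChar, and GetAttachTransform returns a random billboard transform.
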(event `self.ReceiveBeginPlay`
  (for _array_element (`|MakeArray` (`self.SpawnL`) (`self.SpawnM`) (`self.SpawnR`))
    (switch `int` (`KismetMathLibrary.RandomIntegerInRange` 0 2)
      (:`0`
        (bind _returnvalue (`SceneComponent.K2_GetComponentToWorld` _array_element))
        (`self.Spawn Pickups` _returnvalue))
      (:`1`
        (`/Engine/EditorBlueprintResources/StandardMacros.Do N` 2
          (:`Exit`
            (`self.Spawn Blocker1` _returnvalue))))
      (:`2`
        (`/Engine/EditorBlueprintResources/StandardMacros.Do N` 3
          (:`Exit`
            (`self.Spawn Bcloker 2` _returnvalue)))))))

(event `Spawn Pickups`
  (params (SpawnTransform :type "Transform Structure"))
  (bind _returnvalue (`|SpawnActorFromClass` "/Game/Blueprints/Actor/BP_Pickup.BP_Pickup_C" SpawnTransform "Undefined" "OverrideRootScale" null null))
  (`KismetArrayLibrary.Array_Add` (`self.Pickups`) _returnvalue))

(event `self.EndTrigger.OnComponentBeginOverlap`
  (params (OverlappedComponent :type "PrimitiveComponent Object Reference") (OtherActor :type "Actor Object Reference") (OtherComp :type "PrimitiveComponent Object Reference") (OtherBodyIndex :type Integer) (bFromSweep :type Boolean) (SweepResult :type "HitResult Structure (by ref)"))
  (bind _asmy_char (cast `/Game/Blueprints/MyChar` OtherActor)
    (:`then`
      (bind _output_get (set `self.MyCharRef` _asmy_char))
      (bind _asrunner_gm (cast `/Game/Blueprints/GameMode/RunnerGM` (`GameplayStatics.GetGameMode`)))
      (`/Game/Blueprints/GameMode/RunnerGM.AddFloorTile` _asrunner_gm)
      (if (not (`/Game/Blueprints/MyChar.IsDead` _output_get))
        (`|ExecutionSequence`
          (:`then_0`
            (`self.K2_DestroyActor`))
          (:`then_1`
            (for _array_element (`self.Pickups`)
              (`/Engine/EditorBlueprintResources/StandardMacros.IsValid` _array_element
                (:`Is Valid`
                  (`self.K2_DestroyActor` _array_element))))
            (for _array_element_2 (`self.Blocker1`)
              (`/Engine/EditorBlueprintResources/StandardMacros.IsValid` _array_element_2
                (:`Is Valid`
                  (`self.K2_DestroyActor` _array_element_2))))
            (for _array_element_3 (`self.Blocker2`)
              (`/Engine/EditorBlueprintResources/StandardMacros.IsValid` _array_element_3
                (:`Is Valid`
                  (`self.K2_DestroyActor` _array_element_3))))))))
    (:`CastFailed`
      (`KismetSystemLibrary.PrintString` "End" true true (struct :`R` 1.0 :`G` 0.16074 :`A` 1.0)))))

(event `Spawn Blocker1`
  (params (SpawnTransform :type "Transform Structure"))
  (bind _returnvalue (`|SpawnActorFromClass` "/Game/Blueprints/Actor/BP_Blocker1.BP_Blocker1_C" SpawnTransform "Undefined" "OverrideRootScale" null null))
  (`KismetArrayLibrary.Array_Add` (`self.Blocker1`) _returnvalue))

(event `self.DeadTrigger.OnComponentBeginOverlap`
  (params (OverlappedComponent :type "PrimitiveComponent Object Reference") (OtherActor :type "Actor Object Reference") (OtherComp :type "PrimitiveComponent Object Reference") (OtherBodyIndex :type Integer) (bFromSweep :type Boolean) (SweepResult :type "HitResult Structure (by ref)"))
  (bind _asmy_char (cast `/Game/Blueprints/MyChar` OtherActor)
    (:`then`
      (`/Game/Blueprints/MyChar.Death` _asmy_char))
    (:`CastFailed`
      (`KismetSystemLibrary.PrintString` "Dead???" true true (struct :`R` 1.0 :`A` 1.0)))))

(event `Spawn Bcloker 2`
  (params (SpawnTransform :type "Transform Structure"))
  (bind _returnvalue (`|SpawnActorFromClass` "/Game/Blueprints/Actor/BP_Blocker2.BP_Blocker2_C" SpawnTransform "Undefined" "OverrideRootScale" null null))
  (`KismetArrayLibrary.Array_Add` (`self.Blocker2`) _returnvalue))

(fn `GetAttachTransform`
  (returns (AttachTransform :type "Transform Structure"))
  (bind _returnvalue (`KismetMathLibrary.RandomIntegerInRange` (`self.MinInt`) (`self.MaxInt`)))
  (bind _output_get (set `self.IntResult` _returnvalue))
  (`KismetSystemLibrary.PrintString` (`KismetStringLibrary.Conv_IntToString` _output_get))
  (return (`SceneComponent.K2_GetComponentToWorld` (`|GetArrayItem` (`|MakeArray` (`self.Billboard1`) (`self.Billboard2`)) _returnvalue))))

(fn `UserConstructionScript`)