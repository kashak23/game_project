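; Game mode for a runner game that builds the starting stretch of floor from randomly chosen tiles on BeginPlay.
; AddFloorTile spawns a random class from FloorTiles at NextSpawnPoint, then takes the new tile's attach transform as the next spawn point, chaining tiles end to end.
; Failed casts to BP_FloorTiles1 or the player's MyChar only print debug messages.
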(event `self.ReceiveBeginPlay`
  (for _ (range 7)
    (`self.AddFloorTile`)
    (cast `/Game/Blueprints/MyChar` (`GameplayStatics.GetPlayerCharacter` 0)
      (:`CastFailed`
        (`KismetSystemLibrary.PrintString` "GM Failed!" true true (struct :`R` 1.0 :`G` 0.008603 :`A` 1.0))))))

(fn `AddFloorTile`
  (bind _floortiles (`self.FloorTiles`))
  (bind _returnvalue (`|SpawnActorFromClass` (`|GetArrayItem` _floortiles (`KismetMathLibrary.RandomIntegerInRange` 0 (`KismetArrayLibrary.Array_LastIndex` _floortiles))) (`self.NextSpawnPoint`) "Undefined" "OverrideRootScale" null null))
  (bind _asbp_floor_tiles_1 (cast `/Game/Blueprints/Actor/BP_FloorTiles1` _returnvalue)
    (:`then`
      (bind _attachtransform (`/Game/Blueprints/Actor/BP_FloorTiles1.GetAttachTransform` _asbp_floor_tiles_1))
      (set `self.NextSpawnPoint` _attachtransform))
    (:`CastFailed`
      (`KismetSystemLibrary.PrintString` "GM FloorTile"))))

(fn `UserConstructionScript`)